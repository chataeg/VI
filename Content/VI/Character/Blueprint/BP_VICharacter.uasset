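; BP_VICharacter is a character Blueprint that sets up its controls on BeginPlay and hides its first-person mesh, without affecting child components.
; A debug G key handler, marked for removal, lowers Health while it is above zero.
; Each hit plays the Vignette timeline from the start, writing its track to the VignetteAmount parameter in the VIPawn_MPC material parameter collection.
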(event `Key|G`
  (params (Key :type "Key Structure"))
  ;[1 1 1] 제거 예정
  (:`Pressed`
    (if (> (`self.Health`) 0)
      (set `self.Health` (- (`self.Health`) 10))
      (bind (_direction _newtrack_0) (`Timeline|Vignette` :!via `PlayFromStart`)
        (:`Update`
          (`KismetMaterialLibrary.SetScalarParameterValue` "/Game/WeaponAssets/Textures/VIPawn_MPC.VIPawn_MPC" "VignetteAmount" _newtrack_0))))))

(event `self.ReceiveBeginPlay`
  (`self.SetupCharacterControl`)
  (`SceneComponent.SetVisibility` (`self.FirstPersonMesh`) false false))

(fn `UserConstructionScript`)