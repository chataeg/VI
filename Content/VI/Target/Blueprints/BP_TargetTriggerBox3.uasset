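; Trigger volume that activates shooting-range style targets when the player character (VICharacter) walks into it.
; On overlap it calls RecvTriggerd on every BP_FullTarget_Stand03 in the level, then destroys itself so it fires only once.
; An unwired branch holds staged logic for BP_FullTarget_Stand01, picking targets by a number parsed from display names against TargetArray ranges indexed by the character's TriggerIndex.
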(event `self.ReceiveActorBeginOverlap`
  (params (OtherActor :type "Actor Object Reference"))
  (cast `VICharacter` OtherActor)
  (bind _outactors (`GameplayStatics.GetAllActorsOfClass` "/Game/MOUT_Fabrication/Blueprints/Target/BP_FullTarget_Stand03.BP_FullTarget_Stand03_C"))
  (for _array_element _outactors
    (`/Game/MOUT_Fabrication/Blueprints/Target/BP_FullTarget_Stand03.RecvTriggerd` _array_element))
  (`self.K2_DestroyActor`))

(fn `UserConstructionScript`)